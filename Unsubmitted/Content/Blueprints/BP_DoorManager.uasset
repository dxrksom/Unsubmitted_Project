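; BP_DoorManager runs a door dialogue encounter with a 2D friend who may be real or fake.
; Interact toggles the door camera, input lock and dialogue UI.
; On first use, E draws a role sprite from the game mode's pool and picks the matching DataTable, with fakes always getting DT_FakeFriend1.
; A and D show that row's reply and outfit face, set the round to 1, then refresh choices.
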(event `UpdateDialogAndFace`
  (params (NewText :type Text) (NewFace :type "/Game/Blueprints/Dialog/E_Emotion Enum" :default "NewEnumerator0"))
  (bind _asbp_first_person_game_mode (cast `/Game/FirstPerson/Blueprints/BP_FirstPersonGameMode` (`GameplayStatics.GetGameMode`)))
  (`/Game/Blueprints/Dialog/WBP_DialogueUI.UpdateSubtitle` (`self.UI_Ref`) NewText)
  (switch `/Game/Blueprints/Dialog/E_Emotion` NewFace
    (:`NewEnumerator0`
      (bind (_sprite_default _sprite_wtf _sprite_awkward _sprite_tired _sprite_serious _sprite_monster) (break `/Game/Blueprints/Dialog/ST_OutfitSet` (`/Game/FirstPerson/Blueprints/BP_FirstPersonGameMode.CurrentOutfit` _asbp_first_person_game_mode)))
      (`PaperSpriteComponent.SetSprite` (`self.Friend_2D`) _sprite_default))
    (:`NewEnumerator1`
      (`PaperSpriteComponent.SetSprite` (`self.Friend_2D`) _sprite_wtf))
    (:`NewEnumerator2`
      (`PaperSpriteComponent.SetSprite` (`self.Friend_2D`) _sprite_awkward))
    (:`NewEnumerator3`
      (`PaperSpriteComponent.SetSprite` (`self.Friend_2D`) _sprite_tired))
    (:`NewEnumerator4`
      (`PaperSpriteComponent.SetSprite` (`self.Friend_2D`) _sprite_serious))
    (:`NewEnumerator5`
      (`PaperSpriteComponent.SetSprite` (`self.Friend_2D`) _sprite_monster))))

(event `/Game/Blueprints/BPI_Interactable.Interact`
  (bind _returnvalue (`GameplayStatics.GetPlayerController` 0))
  (bind _returnvalue_2 (`GameplayStatics.GetPlayerController` 0))
  (bind _ui_ref (`self.UI_Ref`))
  (`KismetSystemLibrary.PrintString` "door Received!")
  (`/Engine/EditorBlueprintResources/StandardMacros.FlipFlop`
    (:`A`
      (`|ExecutionSequence`
        (:`then_0`
          (`PlayerController.SetViewTargetWithBlend` _returnvalue_2 self 0.5 "VTBlend_Linear" 0.0 false)
          (`Controller.SetIgnoreMoveInput` _returnvalue_2 true)
          (`Controller.SetIgnoreLookInput` _returnvalue_2 true)
          (bind _returnvalue_3 (`|CreateWidget` "/Game/Blueprints/Dialog/WBP_DialogueUI.WBP_DialogueUI_C"))
          (set `self.UI_Ref` _returnvalue_3)
          (`UserWidget.AddToViewport` _returnvalue_3 0)
          (`self.EnableInput` _returnvalue_2)
          (`self.UpdateDialogAndFace` ""))))
    (:`B`
      (`PlayerController.SetViewTargetWithBlend` _returnvalue (`Controller.K2_GetPawn` _returnvalue) 0.5 "VTBlend_Linear" 0.0 false)
      (`Controller.ResetIgnoreMoveInput` _returnvalue)
      (`Controller.ResetIgnoreLookInput` _returnvalue)
      (`/Engine/EditorBlueprintResources/StandardMacros.IsValid` _ui_ref
        (:`Is Valid`
          (`Widget.RemoveFromParent` _ui_ref)
          (`self.DisableInput` self (`GameplayStatics.GetPlayerController` 0)))))))

(event `Key|A`
  (params (Key :type "Key Structure"))
  (:`Pressed`
    (`/Engine/EditorBlueprintResources/StandardMacros.IsValid` (`self.Current_DataTable`)
      (:`Is Valid`
        (bind _returnvalue (`|GetDataTableRow` (`self.Current_DataTable`) (`KismetStringLibrary.Conv_StringToName` (`KismetStringLibrary.Conv_IntToString` (`self.Current_Round`))))
          (:`then`
            (bind (_text_player_a _text_friend_a _face_a) (break `/Game/Blueprints/Dialog/ST_DialogueData` _returnvalue))
            (`self.UpdateDialogAndFace` _text_friend_a _face_a)
            (set `self.Current_Round` (+ 0 1))
            (`self.RefreshChoicesUI`)))))))

(event `RefreshChoicesUI`
  (bind _returnvalue (`|GetDataTableRow` (`self.Current_DataTable`) (`KismetStringLibrary.Conv_StringToName` (`KismetStringLibrary.Conv_IntToString` (`self.Current_Round`))))
    (:`then`
      (bind (_text_player_a _text_friend_a _face_a _text_player_d) (break `/Game/Blueprints/Dialog/ST_DialogueData` _returnvalue))
      (`/Game/Blueprints/Dialog/WBP_DialogueUI.UpdatePlayerChoices` (`self.UI_Ref`) _text_player_a _text_player_d))))

(event `Key|D`
  (params (Key :type "Key Structure"))
  (:`Pressed`
    (`/Engine/EditorBlueprintResources/StandardMacros.IsValid` (`self.Current_DataTable`)
      (:`Is Valid`
        (bind _returnvalue (`|GetDataTableRow` (`self.Current_DataTable`) (`KismetStringLibrary.Conv_StringToName` (`KismetStringLibrary.Conv_IntToString` (`self.Current_Round`))))
          (:`then`
            (bind (_text_player_a _text_friend_a _face_a _text_player_d _text_friend_d _face_d) (break `/Game/Blueprints/Dialog/ST_DialogueData` _returnvalue))
            (`self.UpdateDialogAndFace` _text_friend_d _face_d)
            (set `self.Current_Round` (+ 0 1))
            (`self.RefreshChoicesUI`)))))))

(event `Key|E`
  (params (Key :type "Key Structure"))
  (:`Pressed`
    (`PlayerController.SetViewTargetWithBlend` (`GameplayStatics.GetPlayerController` 0) null 0.5 "VTBlend_Linear" 0.0 false)
    (`CharacterMovementComponent.DisableMovement` (`Character.CharacterMovement` (`GameplayStatics.GetPlayerCharacter` 0)))
    (if (`self.IsGenerated?`)
      (`PaperSpriteComponent.SetSprite` (`self.Friend_2D`) (`self.Current_Door_Sprite`))
      (else
        (bind _asbp_first_person_game_mode (cast `/Game/FirstPerson/Blueprints/BP_FirstPersonGameMode` (`GameplayStatics.GetGameMode`)))
        (bind _pool_roles (`/Game/FirstPerson/Blueprints/BP_FirstPersonGameMode.Pool_Roles` _asbp_first_person_game_mode))
        (set `self.Current_Door_Sprite` (`|GetArrayItem` _pool_roles))
        (`KismetArrayLibrary.Array_Remove` _pool_roles)
        (set `self.IsGenerated?` true)
        (`PaperSpriteComponent.SetSprite` (`self.Friend_2D`) (`self.Current_Door_Sprite`))
        (if (== (`self.Current_Door_Sprite`) (`/Game/FirstPerson/Blueprints/BP_FirstPersonGameMode.Role_RealFriend` _asbp_first_person_game_mode))
          (set `self.Current_DataTable` "/Game/Blueprints/Dialog/DT_RealFriend.DT_RealFriend")
          (elif true
            (set `self.Current_DataTable` "/Game/Blueprints/Dialog/DT_FakeFriend1.DT_FakeFriend1")
            (else
              (set `self.Current_DataTable` "/Game/Blueprints/Dialog/DT_FakeFriend2.DT_FakeFriend2"))))))
    (bind _returnvalue (`|CreateWidget` "/Game/Blueprints/Dialog/WBP_DialogueUI.WBP_DialogueUI_C"))
    (set `self.UI_Ref` _returnvalue)
    (`UserWidget.AddToViewport` _returnvalue 0)
    (`/Game/Blueprints/Dialog/WBP_DialogueUI.UpdateSubtitle` (`self.UI_Ref`) "")
    (`self.RefreshChoicesUI`)))

(fn `UserConstructionScript`)