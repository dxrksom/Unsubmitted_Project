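; BP_LightSwitch is a light switch actor that shows an on-screen prompt while the first-person character is near it.
; Its Box overlap creates a WBP_LightSwitch widget, stores it and adds it to the viewport, then removes it after a validity check when the character leaves.
; The Interact event feeds a FlipFlop with nothing wired to its outputs, so it does not yet switch any light.
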(event `self.Box.OnComponentBeginOverlap`
  (params (OverlappedComponent :type "PrimitiveComponent Object Reference") (OtherActor :type "Actor Object Reference") (OtherComp :type "PrimitiveComponent Object Reference") (OtherBodyIndex :type Integer) (bFromSweep :type Boolean) (SweepResult :type "HitResult Structure (by ref)"))
  (cast `/Game/FirstPerson/Blueprints/BP_FirstPersonCharacter` OtherActor)
  (bind _returnvalue (`|CreateWidget` "/Game/Blueprints/UI/WBP_LightSwitch.WBP_LightSwitch_C"))
  (bind _output_get (set `self.Light_Prompt_Ref` _returnvalue))
  (`UserWidget.AddToViewport` _output_get 0))

(event `self.Box.OnComponentEndOverlap`
  (params (OverlappedComponent :type "PrimitiveComponent Object Reference") (OtherActor :type "Actor Object Reference") (OtherComp :type "PrimitiveComponent Object Reference") (OtherBodyIndex :type Integer))
  (cast `/Game/FirstPerson/Blueprints/BP_FirstPersonCharacter` OtherActor)
  (`/Engine/EditorBlueprintResources/StandardMacros.IsValid` null
    (:`Is Valid`
      (`Widget.RemoveFromParent` (`self.Light_Prompt_Ref`)))))

(event `/Game/Blueprints/BPI_Interactable.Interact`
  (`/Engine/EditorBlueprintResources/StandardMacros.FlipFlop`))

(fn `UserConstructionScript`)