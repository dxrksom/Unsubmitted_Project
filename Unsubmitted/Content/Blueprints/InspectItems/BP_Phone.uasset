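; BP_Phone is an interactable phone that toggles an on-screen phone viewer widget each time Interact fires.
; When not viewing, it creates WBP_PhoneViwer, adds it to the viewport, plays SlideIn and stores the returned animation reference.
; When viewing and that reference is valid, it plays SlideOut, waits briefly, then removes the widget and clears the IsViewing flag.
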(event `/Game/Blueprints/BPI_Interactable.Interact`
  (if (`self.IsViewing?`)
    (`/Engine/EditorBlueprintResources/StandardMacros.IsValid` (`self.Phone_Ref`)
      (:`Is Valid`
        (`UserWidget.PlayAnimation` (stale _returnvalue) (`/Game/Blueprints/InspectItems/WBP_PhoneViwer.SlideOut` (stale _returnvalue)) 0.0 1 "Forward" 1.0 false)
        (`KismetSystemLibrary.Delay` 0.5)
        (`Widget.RemoveFromParent` (stale _returnvalue))
        (set `self.IsViewing?` false)))
    (else
      (bind _returnvalue (`|CreateWidget` "/Game/Blueprints/InspectItems/WBP_PhoneViwer.WBP_PhoneViwer_C"))
      (`UserWidget.AddToViewport` _returnvalue 0)
      (bind _returnvalue_2 (`UserWidget.PlayAnimation` _returnvalue (`/Game/Blueprints/InspectItems/WBP_PhoneViwer.SlideIn` _returnvalue) 0.0 1 "Forward" 1.0 false))
      (set `self.Phone_Ref` _returnvalue_2)
      (set `self.IsViewing?` true))))

(fn `UserConstructionScript`)