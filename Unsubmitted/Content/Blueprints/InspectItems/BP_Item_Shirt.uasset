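; BP_Item_Shirt is an inspectable shirt item that gives the player a close-up view and a thought about it.
; Its PromptZone shows a Thai interact prompt while the first-person character overlaps it.
; Interact uses a FlipFlop: first it blends the view to the item, locks input and blanks the prompt.
; Next it restores view and input, re-shows the prompt and briefly displays ItemThoughtText in a thought widget.
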(event `self.PromptZone.OnComponentBeginOverlap`
  (params (OverlappedComponent :type "PrimitiveComponent Object Reference") (OtherActor :type "Actor Object Reference") (OtherComp :type "PrimitiveComponent Object Reference") (OtherBodyIndex :type Integer) (bFromSweep :type Boolean) (SweepResult :type "HitResult Structure (by ref)"))
  (cast `/Game/FirstPerson/Blueprints/BP_FirstPersonCharacter` OtherActor)
  (bind _returnvalue (`|CreateWidget` "/Game/Blueprints/UI/WBP_InteractPrompt.WBP_InteractPrompt_C"))
  (bind _output_get (set `self.PromptRef` _returnvalue))
  (`TextBlock.SetText` (`/Game/Blueprints/UI/WBP_InteractPrompt.TXT_Prompt` _output_get) "กด [E] เพื่อดูรายละเอียด" :!label _label)
  (`UserWidget.AddToViewport` (`self.PromptRef`) 0))

(event `self.PromptZone.OnComponentEndOverlap`
  (params (OverlappedComponent :type "PrimitiveComponent Object Reference") (OtherActor :type "Actor Object Reference") (OtherComp :type "PrimitiveComponent Object Reference") (OtherBodyIndex :type Integer))
  (cast `/Game/FirstPerson/Blueprints/BP_FirstPersonCharacter` OtherActor)
  (`Widget.RemoveFromParent` (`self.PromptRef`)))

(event `/Game/Blueprints/BPI_Interactable.Interact`
  (bind _returnvalue (`GameplayStatics.GetPlayerController` 0))
  (`|ExecutionSequence`
    (:`then_0`
      (`/Engine/EditorBlueprintResources/StandardMacros.FlipFlop`
        (:`A`
          (`PlayerController.SetViewTargetWithBlend` _returnvalue self 0.5 "VTBlend_Linear" 0.0 false)
          (`Controller.SetIgnoreMoveInput` _returnvalue true)
          (`Controller.SetIgnoreLookInput` _returnvalue true)
          (bind _output_get (set `self.PromptRef` (stale `self.PromptZone.OnComponentBeginOverlap` _returnvalue)))
          (`TextBlock.SetText` (`/Game/Blueprints/UI/WBP_InteractPrompt.TXT_Prompt` _output_get) ""))
        (:`B`
          (`PlayerController.SetViewTargetWithBlend` _returnvalue (`GameplayStatics.GetPlayerCharacter` 0) 0.5 "VTBlend_Linear" 0.0 false)
          (`Controller.ResetIgnoreMoveInput` _returnvalue)
          (`Controller.ResetIgnoreLookInput` _returnvalue)
          (bind _returnvalue_2 (`|CreateWidget` "/Game/Blueprints/UI/WBP_PlayerThought.WBP_PlayerThought_C"))
          (`TextBlock.SetText` (`/Game/Blueprints/UI/WBP_PlayerThought.TXT_Thought` _returnvalue_2) (`self.ItemThoughtText`))
          (`UserWidget.AddToViewport` _returnvalue_2 0)
          (`|ExecutionSequence`
            (:`then_0`
              (goto _label))
            (:`then_1`
              (`KismetSystemLibrary.Delay` 3.0)
              (`Widget.RemoveFromParent` _returnvalue_2))))))))

(fn `UserConstructionScript`
  (`parent.UserConstructionScript`))