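; Inspectable phone item that the first-person character can open and close as an on-screen phone viewer.
; Its prompt zone shows and removes a Thai interaction prompt on overlap.
; Interact toggles on a viewing flag: opening slides in the viewer with an exit prompt.
; Closing, gated on the stored slide-in animation player being valid, slides it out and briefly shows the item's thought text before removing both widgets.
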(event `self.PromptZone.OnComponentBeginOverlap`
  (params (OverlappedComponent :type "PrimitiveComponent Object Reference") (OtherActor :type "Actor Object Reference") (OtherComp :type "PrimitiveComponent Object Reference") (OtherBodyIndex :type Integer) (bFromSweep :type Boolean) (SweepResult :type "HitResult Structure (by ref)"))
  (cast `/Game/FirstPerson/Blueprints/BP_FirstPersonCharacter` OtherActor)
  (bind _promptref (`self.PromptRef`)
    (:`then`
      (`Widget.RemoveFromParent` _promptref))
    (:`else`
      _))
  (bind _returnvalue (`|CreateWidget` "/Game/Blueprints/UI/WBP_InteractPrompt.WBP_InteractPrompt_C"))
  (bind _output_get (set `self.PromptRef` _returnvalue))
  (`TextBlock.SetText` (`/Game/Blueprints/UI/WBP_InteractPrompt.TXT_Prompt` _output_get) "กด [E] เพื่อดูรายละเอียด")
  (`UserWidget.AddToViewport` (`self.PromptRef`) 0))

(event `self.PromptZone.OnComponentEndOverlap`
  (params (OverlappedComponent :type "PrimitiveComponent Object Reference") (OtherActor :type "Actor Object Reference") (OtherComp :type "PrimitiveComponent Object Reference") (OtherBodyIndex :type Integer))
  (cast `/Game/FirstPerson/Blueprints/BP_FirstPersonCharacter` OtherActor)
  (`Widget.RemoveFromParent` (`self.PromptRef`)))

(event `/Game/Blueprints/BPI_Interactable.Interact`
  (if (`self.IsViewing?`)
    (`/Engine/EditorBlueprintResources/StandardMacros.IsValid` (`self.Phone_Ref`)
      (:`Is Valid`
        (`UserWidget.PlayAnimation` (stale _returnvalue_2) (`/Game/Blueprints/InspectItems/WBP_PhoneViwer.SlideOut` (stale _returnvalue_2)) 0.0 1 "Forward" 1.0 false)
        (`Widget.RemoveFromParent` (`self.Text_Phone`))
        (`KismetSystemLibrary.Delay` 0.5)
        (bind _returnvalue (`|CreateWidget` "/Game/Blueprints/UI/WBP_PlayerThought.WBP_PlayerThought_C"))
        (`TextBlock.SetText` (`/Game/Blueprints/UI/WBP_PlayerThought.TXT_Thought` _returnvalue) (`self.ItemThoughtText`))
        (`UserWidget.AddToViewport` _returnvalue 0)
        (`KismetSystemLibrary.Delay` 3.0)
        (`Widget.RemoveFromParent` _returnvalue)
        (`Widget.RemoveFromParent` (stale _returnvalue_2))
        (set `self.IsViewing?` false)))
    (else
      (bind _returnvalue_2 (`|CreateWidget` "/Game/Blueprints/InspectItems/WBP_PhoneViwer.WBP_PhoneViwer_C"))
      (`UserWidget.AddToViewport` _returnvalue_2 0)
      (bind _returnvalue_3 (`UserWidget.PlayAnimation` _returnvalue_2 (`/Game/Blueprints/InspectItems/WBP_PhoneViwer.SlideIn` _returnvalue_2) 0.0 1 "Forward" 1.0 false))
      (set `self.Phone_Ref` _returnvalue_3)
      (set `self.IsViewing?` true)
      (bind _returnvalue_4 (`|CreateWidget` "/Game/Blueprints/UI/WBP_PhoneIn.WBP_PhoneIn_C"))
      (set `self.Text_Phone` _returnvalue_4)
      (`TextBlock.SetText` (`/Game/Blueprints/UI/WBP_PhoneIn.TXT_Prompt` (`self.Text_Phone`)) "กด [E] เพื่ออกจากหน้าจอ")
      (`UserWidget.AddToViewport` (`self.Text_Phone`) 0))))

(fn `UserConstructionScript`
  (`parent.UserConstructionScript`))