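; BP_Bed is the bed that triggers the game's ending, active only while a BP_Friend_InRoom actor exists in the level.
; Its PromptZone shows a sleep prompt widget when the first-person character enters and removes it on exit.
; Interacting disables player input, plays a sleep fade, then after a short delay calls the good or bad ending depending on whether BP_DoorManager's current data table is DT_RealFriend.
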(event `self.PromptZone.OnComponentBeginOverlap`
  (params (OverlappedComponent :type "PrimitiveComponent Object Reference") (OtherActor :type "Actor Object Reference") (OtherComp :type "PrimitiveComponent Object Reference") (OtherBodyIndex :type Integer) (bFromSweep :type Boolean) (SweepResult :type "HitResult Structure (by ref)"))
  (cast `/Game/FirstPerson/Blueprints/BP_FirstPersonCharacter` OtherActor)
  (bind _returnvalue (`GameplayStatics.GetActorOfClass` "/Game/Blueprints/BP_Friend_InRoom.BP_Friend_InRoom_C"))
  (`/Engine/EditorBlueprintResources/StandardMacros.IsValid` _returnvalue
    (:`Is Valid`
      (bind _returnvalue_2 (`|CreateWidget` "/Game/Blueprints/UI/WBP_SleepPrompt.WBP_SleepPrompt_C"))
      (bind _output_get (set `self.UI_Prompt` _returnvalue_2))
      (`UserWidget.AddToViewport` _output_get 0))))

(event `self.PromptZone.OnComponentEndOverlap`
  (params (OverlappedComponent :type "PrimitiveComponent Object Reference") (OtherActor :type "Actor Object Reference") (OtherComp :type "PrimitiveComponent Object Reference") (OtherBodyIndex :type Integer))
  (cast `/Game/FirstPerson/Blueprints/BP_FirstPersonCharacter` OtherActor)
  (`/Engine/EditorBlueprintResources/StandardMacros.IsValid` null
    (:`Is Valid`
      (`Widget.RemoveFromParent` (`self.UI_Prompt`)))))

(event `/Game/Blueprints/BPI_Interactable.Interact`
  (bind _returnvalue (`GameplayStatics.GetActorOfClass` "/Game/Blueprints/BP_Friend_InRoom.BP_Friend_InRoom_C"))
  (`/Engine/EditorBlueprintResources/StandardMacros.IsValid` _returnvalue
    (:`Is Valid`
      (`self.DisableInput` (`GameplayStatics.GetPlayerController` 0))
      (bind _returnvalue_2 (`|CreateWidget` "/Game/Blueprints/Ending/WBP_SleepFade.WBP_SleepFade_C"))
      (`UserWidget.AddToViewport` _returnvalue_2 0)
      (`UserWidget.PlayAnimation` _returnvalue_2 (`/Game/Blueprints/Ending/WBP_SleepFade.Anim_Sleep` _returnvalue_2) 0.0 1 "Forward" 1.0 false)
      (`KismetSystemLibrary.Delay` 3.0)
      (bind _returnvalue_3 (`GameplayStatics.GetActorOfClass` "/Game/Blueprints/BP_DoorManager.BP_DoorManager_C"))
      (if (== (`/Game/Blueprints/BP_DoorManager.Current_DataTable` _returnvalue_3) "/Game/Blueprints/Dialog/DT_RealFriend.DT_RealFriend")
        (`self.Call_GoodEnding`)
        (else
          (`self.Call_BadEnding`))))))

(fn `UserConstructionScript`)