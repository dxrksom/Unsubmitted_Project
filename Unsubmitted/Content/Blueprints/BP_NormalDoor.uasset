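; BP_NormalDoor is a hinged door that the first-person character can open from either side.
; Two trigger boxes show a prompt widget on overlap and set the Inside flag to record the player's side.
; Interact uses that flag to pick a positive or negative yaw target, then the DoorAnim timeline rotates the Hinge and reverses after a delay.
; IsOpen gates Interact and one prompt, but is never set true here.
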(event `self.Box1.OnComponentBeginOverlap`
  (params (OverlappedComponent :type "PrimitiveComponent Object Reference") (OtherActor :type "Actor Object Reference") (OtherComp :type "PrimitiveComponent Object Reference") (OtherBodyIndex :type Integer) (bFromSweep :type Boolean) (SweepResult :type "HitResult Structure (by ref)"))
  (cast `/Game/FirstPerson/Blueprints/BP_FirstPersonCharacter` OtherActor)
  (if (not (`self.IsOpen?`))
    (bind _returnvalue (`|CreateWidget` "/Game/Blueprints/UI/WBP_DoorNormalPrompt.WBP_DoorNormalPrompt_C"))
    (bind _output_get (set `self.UI_Prompt_Ref` _returnvalue))
    (`UserWidget.AddToViewport` _output_get 10)
    (`KismetSystemLibrary.PrintString` "Inside")
    (set `self.Inside?` true)
    (`KismetSystemLibrary.PrintString` (`KismetStringLibrary.Conv_BoolToString` (`self.Inside?`)))))

(event `self.Box1.OnComponentEndOverlap`
  (params (OverlappedComponent :type "PrimitiveComponent Object Reference") (OtherActor :type "Actor Object Reference") (OtherComp :type "PrimitiveComponent Object Reference") (OtherBodyIndex :type Integer))
  (cast `/Game/FirstPerson/Blueprints/BP_FirstPersonCharacter` OtherActor)
  (`/Engine/EditorBlueprintResources/StandardMacros.IsValid` null
    (:`Is Valid`
      (set `self.Inside?` false)
      (`Widget.RemoveFromParent` (`self.UI_Prompt_Ref`)))))

(event `self.Box.OnComponentBeginOverlap`
  (params (OverlappedComponent :type "PrimitiveComponent Object Reference") (OtherActor :type "Actor Object Reference") (OtherComp :type "PrimitiveComponent Object Reference") (OtherBodyIndex :type Integer) (bFromSweep :type Boolean) (SweepResult :type "HitResult Structure (by ref)"))
  (`KismetSystemLibrary.PrintString` "Hello")
  (cast `/Game/FirstPerson/Blueprints/BP_FirstPersonCharacter` OtherActor)
  (bind _returnvalue (`|CreateWidget` "/Game/Blueprints/UI/WBP_DoorNormalPrompt.WBP_DoorNormalPrompt_C"))
  (bind _output_get (set `self.UI_Prompt_Ref` _returnvalue))
  (`UserWidget.AddToViewport` _output_get 10)
  (`KismetSystemLibrary.PrintString` "Ouside")
  (set `self.Inside?` false)
  (`KismetSystemLibrary.PrintString` (`KismetStringLibrary.Conv_BoolToString` (`self.Inside?`))))

(event `self.Box.OnComponentEndOverlap`
  (params (OverlappedComponent :type "PrimitiveComponent Object Reference") (OtherActor :type "Actor Object Reference") (OtherComp :type "PrimitiveComponent Object Reference") (OtherBodyIndex :type Integer))
  (cast `/Game/FirstPerson/Blueprints/BP_FirstPersonCharacter` OtherActor)
  (`/Engine/EditorBlueprintResources/StandardMacros.IsValid` null
    (:`Is Valid`
      (`Widget.RemoveFromParent` (`self.UI_Prompt_Ref`)))))

(event `/Game/Blueprints/BPI_Interactable.Interact`
  (if (`self.IsOpen?`)
    _
    (elif (`self.Inside?`)
      (set `self.TargetAngle` -90.0)
      (bind (_direction _alpha) (`Timeline|DoorAnim` :!via `PlayFromStart` :!label _label)
        (:`Update`
          (`SceneComponent.K2_SetRelativeRotation` (`self.Hinge`) (`KismetMathLibrary.MakeRotator` 0.0 0.0 (`KismetMathLibrary.Lerp` 0.0 (`self.TargetAngle`) _alpha)) false false))
        (:`Finished`
          (set `self.IsOpen?` false)
          (`KismetSystemLibrary.Delay` 3.0)
          (goto _label :!via `Reverse`)))
      (else
        (set `self.TargetAngle` 90.0)
        (goto _label :!via `PlayFromStart`)))))

(fn `UserConstructionScript`)